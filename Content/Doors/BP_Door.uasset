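; BP_Door is an interactable door actor that swings open and closed when the player interacts with it.
; OnInteract toggles the IsOpen flag and plays or reverses the DoorState timeline.
; The timeline's DoorProgress track, scaled by OpenAngle, sets the Door component's relative yaw on each update, with debug prints of both the interaction and progress.
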(event `self.Interactable.OnInteract`
  (params (Interactor :type "InteractorComponent Object Reference") (Interactable :type "InteractableComponent Object Reference"))
  (`KismetSystemLibrary.PrintString` "Door")
  (if (not (`self.IsOpen`))
    (set `self.IsOpen` true)
    (bind (_direction _doorprogress) (`Timeline|DoorState` :!label _label)
      (:`Update`
        (`KismetSystemLibrary.PrintString` (`KismetStringLibrary.Conv_DoubleToString` _doorprogress) true true (struct :`G` 0.66 :`B` 1.0 :`A` 1.0) 0.0)
        (`SceneComponent.K2_SetRelativeRotation` (`self.Door`) (`KismetMathLibrary.MakeRotator` 0.0 0.0 (* _doorprogress (`self.OpenAngle`))) false false)))
    (else
      (set `self.IsOpen` false)
      (goto _label :!via `Reverse`))))

(fn `UserConstructionScript`)