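; Inventory component for the first-person character that manages the player's inventory screen.
; On BeginPlay it caches the owning BP_FirstPersonCharacter, adds the IMC_Inventory Enhanced Input mapping context, and creates a hidden W_InventoryScreen on the player's screen.
; The screen's Inventory widget receives a reference back to this component as its owning inventory.
; The IA_Inventory action toggles the screen by switching its visibility rather than recreating it.
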(event `self.ReceiveBeginPlay`
  (`self.SetupInput`)
  (`self.CreateInventoryScreen`))

(event `EnhancedInput|/Game/Input/Actions/Inventory/IA_Inventory`
  (params (ActionValue :type Boolean) (ElapsedSeconds :type "Float (double-precision)") (TriggeredSeconds :type "Float (double-precision)") (InputAction :type "InputAction Object Reference" :default "/Game/Input/Actions/Inventory/IA_Inventory.IA_Inventory"))
  (:`Triggered`
    (if (not (`Widget.IsVisible` (`self.InventoryScreen`)))
      (`self.ShowInventoryScreen`)
      (else
        (`self.HideInventoryScreen`)))))

(fn `CreateInventoryScreen`
  (bind _asplayer_controller (cast `PlayerController` (`Pawn.GetController` (`self.Owner`))))
  (bind _returnvalue (`|CreateWidget` "/Game/InventoryAndItems/Inventory/W_InventoryScreen.W_InventoryScreen_C" _asplayer_controller))
  (bind _output_get (set `self.InventoryScreen` _returnvalue))
  (`UserWidget.AddToPlayerScreen` _output_get 0)
  (`self.HideInventoryScreen`)
  (`/Game/InventoryAndItems/Inventory/W_Inventory.SetOwningInventory` (`/Game/InventoryAndItems/Inventory/W_InventoryScreen.Inventory` (`self.InventoryScreen`)) self))

(fn `GetEnhancedInputInterface`
  (returns (ReturnValue :type "EnhancedInputLocalPlayerSubsystem Object Reference"))
  (bind _asplayer_controller (cast `PlayerController` (`Pawn.GetController` (`self.Owner`))))
  (return (pcsubsystem `EnhancedInputLocalPlayerSubsystem` _asplayer_controller)))

(fn `HideInventoryScreen`
  (`Widget.SetVisibility` (`self.InventoryScreen`) "Hidden"))

(fn `SetupInput`
  (bind _asbp_first_person_character (cast `/Game/FirstPerson/Blueprints/BP_FirstPersonCharacter` (`self.GetOwner`)))
  (set `self.Owner` _asbp_first_person_character)
  (`EnhancedInputSubsystemInterface.AddMappingContext` (`self.GetEnhancedInputInterface`) "/Game/Input/IMC_Inventory.IMC_Inventory" 0 (struct)))

(fn `ShowInventoryScreen`
  (`Widget.SetVisibility` (`self.InventoryScreen`) "Visible"))