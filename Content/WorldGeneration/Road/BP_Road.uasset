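; BP_Road procedurally extends a road at runtime, spawning one random segment on BeginPlay and another whenever its trigger box is overlapped.
; Each new segment is positioned from the previous segment's RoadEndArrow, offset along its forward vector and yawed -90 degrees.
; The box then moves to the new end arrow in XY, with collision disabled briefly and restored by timer.
; Debug prints report overlaps and spawn locations.
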(event `self.ReceiveBeginPlay`
  (`self.GenerateRoad`))

(event `self.Box.OnComponentBeginOverlap`
  (params (OverlappedComponent :type "PrimitiveComponent Object Reference") (OtherActor :type "Actor Object Reference") (OtherComp :type "PrimitiveComponent Object Reference") (OtherBodyIndex :type Integer) (bFromSweep :type Boolean) (SweepResult :type "HitResult Structure (by ref)"))
  (`KismetSystemLibrary.PrintString` "Overlap")
  (`self.GenerateRoad`))

(fn `CalculateNewRoadSegmentTransform`
  (params (SpawnedSegment :type "/Game/WorldGeneration/Road/Segments/BP_RoadSegment Object Reference"))
  (returns (ReturnValue :type "Transform Structure"))
  (bind _segments (`self.Segments`))
  (bind _relativelocation_x (`KismetMathLibrary.BreakVector` (`SceneComponent.RelativeLocation` (`/Game/WorldGeneration/Road/Segments/BP_RoadSegment.RoadEndArrow` (`local.SpawnedSegment`)))))
  (bind _roadendarrow (`/Game/WorldGeneration/Road/Segments/BP_RoadSegment.RoadEndArrow` (`|GetArrayItem` _segments (`KismetArrayLibrary.Array_LastIndex` _segments))))
  (bind (_returnvalue_roll _returnvalue_pitch _returnvalue_yaw) (`KismetMathLibrary.BreakRotator` (`SceneComponent.K2_GetComponentRotation` _roadendarrow)))
  (bind _returnvalue (- (`SceneComponent.K2_GetComponentLocation` _roadendarrow) (* (`SceneComponent.GetForwardVector` _roadendarrow) (* _relativelocation_x -1.0))))
  (`KismetSystemLibrary.PrintString` (`KismetStringLibrary.Conv_VectorToString` _returnvalue))
  (return (`KismetMathLibrary.MakeTransform` _returnvalue (`KismetMathLibrary.MakeRotator` _returnvalue_roll _returnvalue_pitch (- _returnvalue_yaw 90.0)))))

(fn `CreateRoadSegment`
  (returns (NewSegment :type "/Game/WorldGeneration/Road/Segments/BP_RoadSegment Object Reference"))
  (locals (SpawnTransform :type "Transform Structure") (NewLocalVar :type "Float (double-precision)" :default -300.0))
  (bind _returnvalue (`|SpawnActorFromClass` (`self.RandomRoadSegment`) (`KismetMathLibrary.MakeTransform` (0.0 0.0 0.0)) "Undefined" "MultiplyWithRoot" null null))
  (if (`KismetArrayLibrary.Array_IsEmpty` (`self.Segments`))
    (set `local.SpawnTransform` (`SceneComponent.K2_GetComponentToWorld` (`self.DefaultSceneRoot`)))
    (else
      (set `local.SpawnTransform` (`self.CalculateNewRoadSegmentTransform` _returnvalue))))
  (`self.K2_SetActorTransform` _returnvalue (`local.SpawnTransform`) false false)
  (return _returnvalue))

(fn `EnableBoxCollision`
  (`PrimitiveComponent.SetCollisionEnabled` (`self.Box`) "QueryOnly"))

(fn `GenerateRoad`
  (locals (NewSegment :type "/Game/WorldGeneration/Road/Segments/BP_RoadSegment Object Reference"))
  (bind (_returnvalue_x _returnvalue_y _returnvalue_z) (`KismetMathLibrary.BreakVector` (`SceneComponent.K2_GetComponentLocation` (`self.Box`))))
  (bind (_returnvalue_x_2 _returnvalue_y_2) (`KismetMathLibrary.BreakVector` (`SceneComponent.K2_GetComponentLocation` (`/Game/WorldGeneration/Road/Segments/BP_RoadSegment.RoadEndArrow` (`local.NewSegment`)))))
  (`PrimitiveComponent.SetCollisionEnabled` (`self.Box`) "NoCollision")
  (bind _newsegment (`self.CreateRoadSegment`))
  (bind _output_get (set `local.NewSegment` _newsegment))
  (`KismetArrayLibrary.Array_Add` (`self.Segments`) _output_get)
  (`SceneComponent.K2_SetWorldLocation` (`self.Box`) (`KismetMathLibrary.MakeVector` _returnvalue_x_2 _returnvalue_y_2 _returnvalue_z) false false)
  (`KismetSystemLibrary.K2_SetTimer` null "EnableBoxCollision" 0.05))

(fn `RandomRoadSegment`
  (returns (RoadSegmentClass :type "/Game/WorldGeneration/Road/Segments/BP_RoadSegment Class Reference"))
  (return (`KismetArrayLibrary.Array_Random` (`self.RoadSegmentVariants`))))

(fn `UserConstructionScript`)